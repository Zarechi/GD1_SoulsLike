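; PC_Isaac is the player controller that turns Enhanced Input into movement, camera look and jumping for the controlled pawn.
; On possess it adds the IMC_Isaac mapping context.
; Move input follows the control rotation's forward and right vectors, including pitch, and look feeds yaw and pitch, with InvertCamera flipping the pitch sign.
; Jump starts and stops through a Character cast, so it only affects Character pawns.
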(event Input|EnhancedActionEvents|EnhancedInputActionIA_Move
  (params (ActionValue :type Vector%202D%20Structure) (ElapsedSeconds :type Float%20%28double-precision%29) (TriggeredSeconds :type Float%20%28double-precision%29) (InputAction :type Input%20Action%20Object%20Reference :default "/Game/_GameManager/Inputs/IA_Move.IA_Move"))
  (bind (_x _y) (Math|Vector2D|BreakVector2D ActionValue))
  (bind _returnvalue (Pawn|GetControlRotation :!class /Script/Engine.Controller))
  (Pawn|Input|AddMovementInput (Pawn|GetControlledPawn) (Math|Vector|GetForwardVector _returnvalue) _y false) ; Forward
  (Pawn|Input|AddMovementInput (Pawn|GetControlledPawn) (Math|Vector|GetRightVector _returnvalue) _x false) ; Right
)

(event Input|EnhancedActionEvents|EnhancedInputActionIA_Look
  (params (ActionValue :type Vector%202D%20Structure) (ElapsedSeconds :type Float%20%28double-precision%29) (TriggeredSeconds :type Float%20%28double-precision%29) (InputAction :type Input%20Action%20Object%20Reference :default "/Game/_GameManager/Inputs/IA_Look.IA_Look"))
  (bind (_x _y) (Math|Vector2D|BreakVector2D ActionValue))
  (Class|PlayerController|AddYawInput _x) ; Horizontal Rotation
  (Class|PlayerController|AddPitchInput (* _y (Math|Float|SelectFloat -1.0 1.0 (Variables|Default|GetInvertCamera)))) ; Vertical Rotation
)

(event Input|EnhancedActionEvents|EnhancedInputActionIA_Jump
  (params (ActionValue :type Boolean) (ElapsedSeconds :type Float%20%28double-precision%29) (TriggeredSeconds :type Float%20%28double-precision%29) (InputAction :type Input%20Action%20Object%20Reference :default "/Game/_GameManager/Inputs/IA_Jump.IA_Jump"))
  (:Triggered
    (bind _ascharacter (Utilities|Casting|CastToCharacter (Pawn|GetControlledPawn)))
    (Character|Jump _ascharacter))
  (:Completed
    (bind _ascharacter_2 (Utilities|Casting|CastToCharacter (Pawn|GetControlledPawn)))
    (Character|StopJumping _ascharacter_2)))

(event EventPossess
  (params (PossessedPawn :type Pawn%20Object%20Reference))
  (bind _returnvalue (PlayerController|LocalPlayerSubsystems|GetEnhancedInputLocalPlayerSubsystem))
  (Utilities|IsValid _returnvalue
    (:Is%20Valid
      (Input|AddMappingContext _returnvalue "/Game/_GameManager/Inputs/IMC_Isaac.IMC_Isaac" 0 "(bIgnoreAllPressedKeysUntilRelease=True,bForceImmediately=False,bNotifyUserSettings=False)"))))

(fn ConstructionScript)