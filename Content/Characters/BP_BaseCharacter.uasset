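; Base character Blueprint that initializes health, endurance, mana and movement speed for characters derived from it.
; On BeginPlay it fills current HP, endurance and mana from their maximums and sets the movement component's walk speed to RunSpeed.
; Tick prints current HP to the screen every frame as debug output, and the construction script is empty.
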(event EventBeginPlay
  (Variables|Stats|Health|SetCurrentHP (Variables|Stats|Health|GetMaxHP))
  (Variables|Stats|Endurance|SetCurrentEndurance (Variables|Stats|Endurance|GetMaxEndurance))
  (Variables|Stats|Mana|SetCurrentMana (Variables|Stats|Mana|GetMaxMana))
  (Variables|/Script/Engine.CharacterMovementComponent|SetMaxWalkSpeed (Variables|Character|GetCharacterMovement) (Variables|Stats|Speed|GetRunSpeed)))

(event EventTick
  (params (DeltaSeconds :type Float%20%28single-precision%29))
  (Development|PrintString (Utilities|String|ToString(Float) (Variables|Stats|Health|GetCurrentHP))))

(fn ConstructionScript)